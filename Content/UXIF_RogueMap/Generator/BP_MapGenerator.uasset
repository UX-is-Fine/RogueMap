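; BP_MapGenerator builds a random roguelike node map, returned as per-tier node data through the overridable GetMapInfo.
; CreatePaths random-walks several paths across tiers, stepping to neighboring positions and filtering against recorded transitions to limit crossovers, staying put if none are safe.
; GetTierData merges each tier's transitions into unique nodes with destination lists.
; GetNodeType fixes certain tiers to Battle, Treasure or Camp and draws others from a probability-weighted pool.
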(fn GetMapInfo
  (CallFunction|CreatePaths) ; override to change logic
  (bind _outtierdata (CallFunction|GetTierData)) ; override to change output
  (return _outtierdata))

(fn CreatePaths
  (bind _rowtransitions (Variables|Default|GetRowTransitions))
  (Utilities|FlowControl|Sequence
    (:then_0
      ;[1 1 1] Init
      (for _index (range 0 (- (Variables|Default|GetNumPaths) 1))
        (LocalVariables|SetiPos (Math|Random|RandomInteger (Variables|Default|GetNumPositions)))
        (Utilities|Array|Add (Variables|Default|GetPaths) (Utilities|Struct|MakeF_Path (Utilities|Array|MakeArray (LocalVariables|GetiPos))))))
    (:then_1
      (Utilities|Array|Resize (Variables|Default|GetRowTransitions) (Variables|Default|GetNumTiers)))
    (:then_2
      ;[1 1 1] For each tier (we will loop paths and determine next location)
      (for _index_2 (range 0 (- (Variables|Default|GetNumTiers) 1))
        (LocalVariables|SetlTier _index_2)
        ;[1 1 1] For each path, we will store current position to determine next location
        (for (_array_element _array_index) (Variables|Default|GetPaths)
          (LocalVariables|SetlCurrentPathIndex _array_index)
          (LocalVariables|SetlCurrentPosition (Utilities|Array|Get(acopy) (Utilities|Struct|BreakF_Path _array_element) (Utilities|Array|LastIndex (Utilities|Struct|BreakF_Path _array_element))))
          ;[1 1 1] Determine safe path destinations
          (LocalVariables|SetlCandidatePositions (CallFunction|GetValidCandidates (LocalVariables|GetlCurrentPosition)))
          (Utilities|Array|Clear (LocalVariables|GetlSafePositions))
          (for _array_element_2 (LocalVariables|GetlCandidatePositions)
            (LocalVariables|SetlCandidate _array_element_2)
            (if (Utilities|Array|IsValidIndex _rowtransitions (LocalVariables|GetlTier))
              (LocalVariables|SetIsSafe true)
              (bind _array_element_3 (Utilities|Array|ForEachLoopwithBreak (Utilities|Struct|BreakF_RowTransitions (Utilities|Array|Get(acopy) _rowtransitions (LocalVariables|GetlTier))) :!label _label)
                (:LoopBody
                  (LocalVariables|SetlSrc (Math|Float|Truncate (.X (Math|Vector2D|BreakVector2D _array_element_3))))
                  (LocalVariables|SetlDst (Math|Float|Truncate (.Y (Math|Vector2D|BreakVector2D _array_element_3))))
                  (if (and (== (Math|Integer|Absolute(Integer) (- (LocalVariables|GetlCandidate) (LocalVariables|GetlDst))) 1) (<= (Math|Integer|Absolute(Integer) (- (LocalVariables|GetlCurrentPosition) (LocalVariables|GetlSrc))) 1))
                    (LocalVariables|SetIsSafe false)
                    (goto _label Break)))
                (:Completed
                  (if (LocalVariables|GetIsSafe)
                    (Utilities|Array|Add (LocalVariables|GetlSafePositions) (LocalVariables|GetlCandidate)))))
              (else
                (Development|PrintString 0 "F"))))
          ;[1 1 1] Set Chosen Position
          (if (Utilities|Array|IsNotEmpty (LocalVariables|GetlSafePositions))
            (LocalVariables|SetlChosenPosition (.OutItem (Utilities|Array|Random (LocalVariables|GetlSafePositions))))
            (else
              (LocalVariables|SetlChosenPosition (LocalVariables|GetlCurrentPosition))))
          ;[1 1 1] Update Used Transitions
          (bind _output_get (LocalVariables|SetiFromTo (Utilities|Struct|BreakF_RowTransitions (Utilities|Array|Get(acopy) (Variables|Default|GetRowTransitions) (LocalVariables|GetlTier)))))
          (Utilities|Array|Add _output_get (Math|Vector2D|MakeVector2D (Math|Conversions|ToFloat(Integer) (LocalVariables|GetlCurrentPosition)) (Math|Conversions|ToFloat(Integer) (LocalVariables|GetlChosenPosition))))
          (Utilities|Array|SetArrayElem (Variables|Default|GetRowTransitions) (LocalVariables|GetlTier) (Utilities|Struct|MakeF_RowTransitions (LocalVariables|GetiFromTo)) true)
          ;[1 1 1] Apply Destination to paths
          (LocalVariables|SetlCurrentPathPositions (Utilities|Struct|BreakF_Path (Utilities|Array|Get(acopy) (Variables|Default|GetPaths) (LocalVariables|GetlCurrentPathIndex))))
          (Utilities|Array|Add (LocalVariables|GetlCurrentPathPositions) (LocalVariables|GetlChosenPosition))
          ;[1 1 1] Update Path
          (Utilities|Array|SetArrayElem (Variables|Default|GetPaths) (LocalVariables|GetlCurrentPathIndex) (Utilities|Struct|MakeF_Path (LocalVariables|GetlCurrentPathPositions))))))))

(fn GetValidCandidates
  (params (Current :type Integer))
  (bind _output_get (LocalVariables|SetlCandidates (Utilities|Array|MakeArray (- Current 1) Current (+ Current 1))))
  (bind (_arrayindex _arrayelement) (Utilities|Array|ReverseforEachLoop _output_get)
    (:LoopBody
      (if (or (< _arrayelement 0) (> _arrayelement (- (Variables|Default|GetNumPositions) 1)))
        (Utilities|Array|RemoveIndex (LocalVariables|GetlCandidates) _arrayindex)))
    (:Completed
      (return (LocalVariables|GetlCandidates)))))

(fn GetTierData
  ;[1 1 1] For each transition in a row, create unique nodes with destinations
  (for (_array_element _array_index) (Variables|Default|GetRowTransitions)
    (LocalVariables|SetlTier _array_index)
    (Utilities|Array|Clear (LocalVariables|GetlNodes))
    (for _array_element_2 (Utilities|Struct|BreakF_RowTransitions _array_element)
      (LocalVariables|SetiPosition (Math|Float|Truncate (.X (Math|Vector2D|BreakVector2D _array_element_2))))
      ;[1 1 1] Add a Node for each unique Position, and apply all destinations from the Transitions list
      (LocalVariables|SetlFoundNode false)
      (for _array_element_3 (LocalVariables|GetlNodes)
        (if (== (Utilities|Struct|BreakF_MapNode _array_element_3) (LocalVariables|GetiPosition))
          (LocalVariables|SetlFoundNode true)))
      (if (not (LocalVariables|GetlFoundNode))
        (Utilities|Array|Clear (LocalVariables|GetlDestinations))
        (for _array_element_4 (Utilities|Struct|BreakF_RowTransitions (Utilities|Array|Get(acopy) (Variables|Default|GetRowTransitions) (LocalVariables|GetlTier)))
          (if (== (.X (Math|Vector2D|BreakVector2D _array_element_4)) (LocalVariables|GetiPosition))
            (Utilities|Array|AddUnique (LocalVariables|GetlDestinations) (Math|Float|Truncate (.Y (Math|Vector2D|BreakVector2D _array_element_4))))))
        (Utilities|Array|Add (LocalVariables|GetlNodes) (Utilities|Struct|MakeF_MapNode (LocalVariables|GetlTier) (LocalVariables|GetiPosition) (CallFunction|GetNodeType (LocalVariables|GetlTier)) (LocalVariables|GetlDestinations)))))
    ;[1 1 1] Add these nodes as a tier
    (Utilities|Array|Add (LocalVariables|GetlTierData) (Utilities|Struct|MakeF_MapTier (LocalVariables|GetlNodes))))
  ;[1 1 1] Return Node Data Per Tier
  (return (LocalVariables|GetlTierData)))

(fn GetNodeType
  (params (Tier :type Integer))
  (bind _lnodepool (LocalVariables|GetlNodePool))
  (Utilities|FlowControl|Sequence
    (:then_0
      ;[1 1 1] Tier 1 always Battle
      (if (== Tier 0)
        (return "/Game/UXIF_RogueMap/Nodes/DA_MapNode_Battle.DA_MapNode_Battle")))
    (:then_1
      ;[1 1 1] Tier 9 always Treasure
      (if (== Tier 4)
        (return "/Game/UXIF_RogueMap/Nodes/DA_MapNode_Treasure.DA_MapNode_Treasure")))
    (:then_2
      ;[1 1 1] Tier 14 always Rest
      (if (== Tier 7)
        (return "/Game/UXIF_RogueMap/Nodes/DA_MapNode_Camp.DA_MapNode_Camp")))
    (:then_3
      ;[1 1 1] Random node
      (for _array_element (Variables|Default|GetNodeTypes)
        (for _index (range 0 (- (Variables|/Game/UXIF_RogueMap/Nodes/Data_MapNode.Data_MapNode_C|GetProbability _array_element) 1))
          (Utilities|Array|Add (LocalVariables|GetlNodePool) _array_element)))
      (Utilities|Array|Shuffle _lnodepool)
      (return (.OutItem (Utilities|Array|Random _lnodepool))))))