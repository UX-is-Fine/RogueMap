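; Actor component that manages save data for the rogue-style node map, storing the current map, current node and player route.
; GetSaveData returns a cached save object, loading it from the slot on first use and creating a new one if missing, deleting any save that fails to load or cast.
; SetNode and SetMap write to disk immediately, while ResetSave deletes the slot and clears the cache.
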(fn GetSaveData
  (bind _loadedsavedata (Variables|Default|GetLoadedSaveData)
    (:then
      (return _loadedsavedata))
    (:else
      (bind _returnvalue (Core|LoadSaveData))
      (bind _output_get (Variables|Default|SetLoadedSaveData _returnvalue))
      (return _output_get))))

(fn LoadSaveData
  (bind _returnvalue (SaveGame|DoesSaveGameExist (Variables|Default|GetSlotName)))
  (if _returnvalue
    (bind _returnvalue_2 (SaveGame|LoadGamefromSlot (Variables|Default|GetSlotName)))
    (Utilities|IsValid _returnvalue_2
      (:Is%20Valid
        (bind _asbp_save_game_node_map (Utilities|Casting|CastToBP_SaveGame_NodeMap _returnvalue_2)
          (:then
            (return _asbp_save_game_node_map))
          (:CastFailed
            _)))
      (:Is%20Not%20Valid
        _))
    (SaveGame|DeleteGameinSlot (Variables|Default|GetSlotName)))
  (bind _returnvalue_3 (Core|CreateSaveData))
  (return _returnvalue_3))

(fn CreateSaveData
  (bind _returnvalue (SaveGame|CreateSaveGameObject "/Game/UXIF_RogueMap/NodeMapSaveData/BP_SaveGame_NodeMap.BP_SaveGame_NodeMap_C"))
  (Core|SaveData _returnvalue)
  (return _returnvalue))

(fn SetNode
  (params (NewNode :type F%20Map%20Node%20Structure))
  (bind _savedata (Core|GetSaveData))
  (bind _output_get (Variables|/Game/UXIF_RogueMap/NodeMapSaveData/BP_SaveGame_NodeMap.BP_SaveGame_NodeMap_C|SetCurrentNode _savedata NewNode))
  (Utilities|Array|Add (Variables|/Game/UXIF_RogueMap/NodeMapSaveData/BP_SaveGame_NodeMap.BP_SaveGame_NodeMap_C|GetPlayerRoute _savedata) _output_get)
  (Core|SaveData _savedata))

(fn SetMap
  (params (CurrentMap :type Array%20of%20F%20Map%20Tier%20Structures))
  (bind _savedata (Core|GetSaveData))
  (Variables|/Game/UXIF_RogueMap/NodeMapSaveData/BP_SaveGame_NodeMap.BP_SaveGame_NodeMap_C|SetCurrentMap _savedata CurrentMap)
  (Core|SaveData _savedata))

(fn SaveData
  (params (SaveGameObject :type Save%20Game%20Object%20Reference))
  (SaveGame|SaveGametoSlot SaveGameObject (Variables|Default|GetSlotName)))

(fn ResetSave
  (SaveGame|DeleteGameinSlot (Variables|Default|GetSlotName))
  (Variables|Default|SetLoadedSaveData 0))